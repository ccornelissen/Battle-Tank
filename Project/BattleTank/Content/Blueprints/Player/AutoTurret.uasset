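; Auto turret pawn that starts neutral and is captured for the red or blue team by a tank staying in its capture zone.
; On BeginPlay it sets up the aiming component, marks its tank AI controller neutral and has it find the nearest tank.
; Overlap on the Cube starts a Tick timer; after three seconds it copies the overlapping tank's team, recolors turret and zone, and retargets.
; Ending the overlap resets the timer.
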(event `self.ReceiveBeginPlay`
  (`TankAimingComponent.Initialize` (`self.TurretAiming`) (`self.TurretBarrel`) (`self.TurretDome`))
  (bind _astank_aicontroller_bp (cast `/Game/Blueprints/Player/TankAIController_BP` (`self.GetController`))
    (:`then`
      (bind _output_get (set `self.OwningController` _astank_aicontroller_bp))
      (set `TankAIController.AITeam` "AT_Neutral" _output_get)
      (`self.ChangeColor` "/Game/Material/M_Metal_Steel.M_Metal_Steel")
      (`TankAIController.GetNearestTank` (`self.OwningController`)))
    (:`CastFailed`
      (`KismetSystemLibrary.PrintString` "Tank Turret Lacking Controller"))))

(event `self.ReceiveTick`
  (params (DeltaSeconds :type "Float (single-precision)"))
  ;[1 1 1] Tick and change components team and color based on overlapp collsion events
  (if (`self.ShouldTick`)
    (set `self.ChangeTimer` (+ (`self.ChangeTimer`) (* 1.0 DeltaSeconds)))
    (if (<= 3.0 (`self.ChangeTimer`))
      (set `TankAIController.AITeam` (select `ETankTeam` (`Tank.TankTeam` (`self.OverlapTank`)) :`TT_Blue` "AT_Blue" :`TT_Red` "AT_Red" :!type "EAITeam Enum") (`self.OwningController`))
      (`self.ChangeColor` (select `ETankTeam` (`Tank.TankTeam` (`self.OverlapTank`)) :`TT_Blue` "/Game/Material/Tank/M_Metal_Steel_Blue.M_Metal_Steel_Blue" :`TT_Red` "/Game/Material/Tank/M_Metal_Steel_Red.M_Metal_Steel_Red" :!type "MaterialInterface Object Reference"))
      (`PrimitiveComponent.SetMaterial` (`self.Cube`) 0 (select `ETankTeam` (`Tank.TankTeam` (`self.OverlapTank`)) :`TT_Blue` "/Game/Material/TurretCaptureZone/Blue_M.Blue_M" :`TT_Red` "/Game/Material/TurretCaptureZone/Red_M.Red_M" :!type "MaterialInterface Object Reference"))
      (`TankAIController.GetNearestTank` (`self.OwningController`)))))

(event `self.Cube.OnComponentBeginOverlap`
  (params (OverlappedComponent :type "PrimitiveComponent Object Reference") (OtherActor :type "Actor Object Reference") (OtherComp :type "PrimitiveComponent Object Reference") (OtherBodyIndex :type Integer) (bFromSweep :type Boolean) (SweepResult :type "HitResult Structure (by ref)"))
  ;[1 1 1] Set the change timer and get the overlapping actor
  (set `self.ShouldTick` true)
  (bind _astank_bp (cast `/Game/Blueprints/Player/Tank_BP` OtherActor))
  (set `self.OverlapTank` _astank_bp))

(event `self.Cube.OnComponentEndOverlap`
  (params (OverlappedComponent :type "PrimitiveComponent Object Reference") (OtherActor :type "Actor Object Reference") (OtherComp :type "PrimitiveComponent Object Reference") (OtherBodyIndex :type Integer))
  ;[1 1 1] Set the change timer and get the overlapping actor
  (set `self.ChangeTimer` 0.0)
  (set `self.ShouldTick` false))

(fn `ChangeColor`
  (params (NewColor :type "MaterialInterface Object Reference"))
  (`PrimitiveComponent.SetMaterial` (`self.TurretBarrel`) 0 NewColor)
  (`PrimitiveComponent.SetMaterial` (`self.TurretDome`) 0 NewColor)
  (`PrimitiveComponent.SetMaterial` (`self.TurretBody`) 0 NewColor))

(fn `UserConstructionScript`)