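; Player controller for a tank that manages the player's UI widget.
; On BeginPlay it creates PlayerUI owned by player controller index 1, adds it to that player's screen and hides the controlled Tank_BP's health bar.
; FoundAimingComponent passes the tank's aiming component to the widget, and TankDeath hides and disables the widget.
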(event `self.TankDeath`
  (params (Location :type "Vector Structure") (Rotation :type "Rotator Structure"))
  (`Widget.SetVisibility` (stale `self.ReceiveBeginPlay` _returnvalue) "Hidden")
  (`Widget.SetIsEnabled` (stale `self.ReceiveBeginPlay` _returnvalue) false))

(event `self.ReceiveBeginPlay`
  (bind _returnvalue (`|CreateWidget` "/Game/Blueprints/Player/PlayerUI.PlayerUI_C" (`GameplayStatics.GetPlayerController` 1)))
  (`UserWidget.AddToPlayerScreen` _returnvalue 0)
  (bind _astank_bp (cast `/Game/Blueprints/Player/Tank_BP` (`self.K2_GetPawn`)))
  (`SceneComponent.SetVisibility` (`/Game/Blueprints/Player/Tank_BP.HealthBar` _astank_bp) false false))

(event `self.FoundAimingComponent`
  (params (AimingComponent :type "TankAimingComponent Object Reference"))
  (set `/Game/Blueprints/Player/PlayerUI.TankAimingComponent` AimingComponent (stale `self.ReceiveBeginPlay` _returnvalue)))

(fn `UserConstructionScript`)