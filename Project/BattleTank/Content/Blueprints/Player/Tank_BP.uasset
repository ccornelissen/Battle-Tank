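; Player tank Blueprint that handles orbit-style camera aiming and quitting to the main menu.
; On BeginPlay it hands its barrel and turret components to the SetBarrelReference and SetTurretReference functions.
; Azimuth input yaws a gimbal, while elevation input pitches the spring arm in world space within a clamped range, both scaled by frame time.
; Releasing Quit opens the MainMenu level.
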(event `self.ReceiveBeginPlay`
  (`self.SetBarrelReference` (`self.TankBarrel`))
  (`self.SetTurretReference` (`self.TankTurret`)))

(event `InputAxis|AimAzimuth`
  (params (AxisValue :type "Float (single-precision)"))
  ;[1 1 1] Camera Z Axis Movement
  (`SceneComponent.K2_AddLocalRotation` (`self.AzimuthGimble`) (`KismetMathLibrary.MakeRotator` 0.0 0.0 (* AxisValue (`GameplayStatics.GetWorldDeltaSeconds`) 100.0)) false false))

(event `InputAxis|AimElevation`
  (params (AxisValue :type "Float (single-precision)"))
  ;[1 1 1] Camera Y Axis Movement
  (`SceneComponent.K2_SetWorldRotation` (`self.SpringArm`) (`KismetMathLibrary.MakeRotator` (.roll (`SceneComponent.K2_GetComponentRotation` (`self.SpringArm`))) (`KismetMathLibrary.FClamp` (+ (.pitch (`SceneComponent.K2_GetComponentRotation` (`self.SpringArm`))) (* AxisValue (`GameplayStatics.GetWorldDeltaSeconds`) 100.0)) -40.0 40.0) (.yaw (`SceneComponent.K2_GetComponentRotation` (`self.SpringArm`)))) false false))

(event `InputAction|Quit`
  (params (Key :type "Key Structure" :default "AnyKey"))
  (:`Released`
    (`GameplayStatics.OpenLevel` "MainMenu")))

(fn `UserConstructionScript`)